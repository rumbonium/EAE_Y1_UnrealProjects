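; Player pawn that moves with axis input, jumps, tracks score and reloads the current level on death.
; Movement input follows actor forward and right vectors, while jumping applies an upward force to the mesh, gated by a grounded flag that straight-up hit normals restore.
; It creates the score HUD on begin play and updates it from AddScore.
; The P key opens a reused pause menu, pausing the game with UI-only input.
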(event `self.ReceiveHit`
  (params (MyComp :type "PrimitiveComponent Object Reference") (Other :type "Actor Object Reference") (OtherComp :type "PrimitiveComponent Object Reference") (bSelfMoved :type Boolean) (HitLocation :type "Vector Structure") (HitNormal :type "Vector Structure") (NormalImpulse :type "Vector Structure") (Hit :type "HitResult Structure (by ref)"))
  ;[1 1 1] Ground Checking
  (if (== HitNormal (0.0 0.0 1.0))
    (set `self.Grounded` true)))

(event `InputAxis|Move_ForwardBack`
  (params (AxisValue :type "Float (single-precision)"))
  ;[1 1 1] Movement
  (`self.AddMovementInput` (`self.GetActorForwardVector`) AxisValue))

(event `Key|P`
  (params (Key :type "Key Structure"))
  (bind _returnvalue (`GameplayStatics.GetPlayerController` 0))
  (bind _pausemenureference (`self.PauseMenuReference`))
  (:`Pressed`
    (`/Engine/EditorBlueprintResources/StandardMacros.IsValid` (`self.PauseMenuReference`)
      (:`Is Valid`
        _)
      (:`Is Not Valid`
        (bind _returnvalue_2 (`|CreateWidget` "/Game/Blueprints/PauseMenu.PauseMenu_C"))
        (set `self.PauseMenuReference` _returnvalue_2)))
    (set `PlayerController.bShowMouseCursor` true _returnvalue)
    (`WidgetBlueprintLibrary.SetInputMode_UIOnlyEx` _returnvalue _pausemenureference)
    (`UserWidget.AddToViewport` _pausemenureference 0)
    (`GameplayStatics.SetGamePaused` true)))

(event `InputAxis|Move_LeftRight`
  (params (AxisValue :type "Float (single-precision)"))
  ;[1 1 1] Movement
  (`self.AddMovementInput` (`self.GetActorRightVector`) AxisValue))

(event `InputAction|Jump`
  (params (Key :type "Key Structure"))
  ;[1 1 1] Jumping
  (:`Pressed`
    (if (`self.Grounded`)
      (`PrimitiveComponent.AddForce` (`self.StaticMesh`) (* (`KismetMathLibrary.Vector_Up`) (`self.jumpForce`)) "None" true)
      (set `self.Grounded` false))))

(event `self.ReceiveBeginPlay`
  (bind _returnvalue (`GameplayStatics.GetPlayerController` 0))
  (bind _returnvalue_2 (`|CreateWidget` "/Game/Blueprints/ScoreUI.ScoreUI_C" _returnvalue))
  (`UserWidget.AddToViewport` _returnvalue_2 0)
  (set `self.ScoreUI` _returnvalue_2)
  (`WidgetBlueprintLibrary.SetInputMode_GameOnly` _returnvalue))

(fn `AddScore`
  (params (ScoreToGive :type Integer))
  (bind _output_get (set `self.Score` (+ ScoreToGive (`self.Score`))))
  (`/Game/Blueprints/ScoreUI.UpdateScore` (`self.ScoreUI`) _output_get))

(fn `Die`
  (bind _returnvalue (`GameplayStatics.GetCurrentLevelName` true))
  (`GameplayStatics.OpenLevel` (`KismetStringLibrary.Conv_StringToName` _returnvalue)))

(fn `UserConstructionScript`)

(fn `ViewUI`
  (`UserWidget.AddToViewport` (`self.ScoreUI`) 0))