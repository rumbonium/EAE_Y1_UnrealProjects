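; Build-a-gun button actor that marks itself as the single active unique mod when another actor overlaps it.
; On overlap it turns every point light in its target light array red and clears the active flag on every button in its button array.
; It then turns the light at its own index green and sets itself active, giving radio-button style exclusive selection.
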(event `self.ReceiveActorBeginOverlap`
  (params (OtherActor :type "Actor Object Reference"))
  (for _array_element (`self.TargetLightArray`)
    (`LightComponent.SetLightColor` (`self.GetComponentByClass` _array_element "/Script/Engine.PointLightComponent") (make `LinearColor` 1.0 0.0 0.0 1.0) true))
  (for _array_element_2 (`self.UniqueButtonArray`)
    (bind _asactivate_unique_mod_button_blueprint (cast `/Game/BuildAGun/Blueprints/ActivateUniqueMod_Button_Blueprint` _array_element_2))
    (set `/Game/BuildAGun/Blueprints/ActivateUniqueMod_Button_Blueprint.IsActive` false _asactivate_unique_mod_button_blueprint))
  (`LightComponent.SetLightColor` (`self.GetComponentByClass` (`|GetArrayItem` (`self.TargetLightArray`) (`self.Index`)) "/Script/Engine.PointLightComponent") (make `LinearColor` 0.0 1.0 0.0 1.0) true)
  (set `self.IsActive` true))

(fn `UserConstructionScript`)