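; BP_Cannon is a cannon actor that automatically and repeatedly fires projectiles from the moment play begins.
; After each FireRate delay, it spawns a BP_Projectile at the ProjectileSpawnPoint transform, scaled by ProjectileScale.
; A timeline then animates the barrel along its relative Y axis, and its Cannon Fired event track restarts the delay to close the loop.
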(event `self.ReceiveBeginPlay`
  (`KismetSystemLibrary.Delay` (`self.FireRate`) :!label _label)
  (`self.SpawnProjectile`)
  (bind (_direction _cannonbarrellocation) (`Timeline|CannonBarrelAnimationTimeline` :!via `PlayFromStart`)
    (:`Update`
      (`self.MoveCannonBarrel` _cannonbarrellocation))
    (:`CannonFired`
      (goto _label))))

(fn `MoveCannonBarrel`
  (params (CannonBarrel_Y :type "Float (double-precision)"))
  (`SceneComponent.K2_SetRelativeLocation` (`self.CannonBarrel`) (`KismetMathLibrary.MakeVector` 0.0 CannonBarrel_Y) false false))

(fn `SpawnProjectile`
  (bind _projectilespawnpoint (`self.ProjectileSpawnPoint`))
  (`|SpawnActorFromClass` "/Game/Blueprints/Actors/Projectiles/BP_Projectile.BP_Projectile_C" (`KismetMathLibrary.MakeTransform` (`SceneComponent.K2_GetComponentLocation` _projectilespawnpoint) (`SceneComponent.K2_GetComponentRotation` _projectilespawnpoint) (`KismetMathLibrary.Conv_DoubleToVector` (`self.ProjectileScale`))) "Undefined" "OverrideRootScale" null null)
  (return))

(fn `UserConstructionScript`)